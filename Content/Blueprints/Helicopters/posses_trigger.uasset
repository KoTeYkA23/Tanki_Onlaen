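; A one-shot trigger actor in the helicopters folder that hands control of a preset pawn to whoever walks or moves into it.
; On overlap, it ignores Helicopter1 actors and requires a valid PawnToPosses and instigator controller.
; That controller possesses the pawn, then the overlapping actor and the trigger are both destroyed.
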(event Collision|EventActorBeginOverlap
  (params (OtherActor :type Actor%20Object%20Reference))
  (bind _returnvalue (Game|GetInstigatorController OtherActor))
  (bind _pawn_to_posses (Variables|Default|Getpawn%20to%20posses))
  (if (and true (!= (Utilities|GetClass OtherActor) "/Game/Blueprints/Helicopters/Helicopter1.Helicopter1_C"))
    (Utilities|IsValid _pawn_to_posses
      (:Is%20Valid
        (Utilities|IsValid _returnvalue
          (:Is%20Valid
            (Pawn|Possess _returnvalue _pawn_to_posses)
            (Actor|DestroyActor OtherActor)
            (Actor|DestroyActor)))))))

(fn ConstructionScript)