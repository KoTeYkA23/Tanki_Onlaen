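; Explosion range actor in the helicopter folder that sizes a sphere component and a particle effect from a Range variable.
; Range sets the sphere radius and multiplies the particle system's relative scale by its ratio to a 64-unit base.
; Both the construction script and BeginPlay run this sizing, so the multiplicative particle scaling can compound at play.
; The graphs contain no damage or overlap handling.
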(event EventBeginPlay
  (bind _range (Variables|Default|Getrange))
  (bind _particlesystem (Variables|Default|GetParticleSystem))
  (Components|Sphere|SetSphereRadius (Variables|Default|GetSphere) _range true)
  (Transformation|SetRelativeScale3D _particlesystem (* (Variables|/Script/Engine.SceneComponent|GetRelativeScale3D _particlesystem) (/ _range 64.0))))

(fn ConstructionScript
  (bind _range (Variables|Default|Getrange))
  (bind _particlesystem (Variables|Default|GetParticleSystem))
  (Components|Sphere|SetSphereRadius (Variables|Default|GetSphere) _range true)
  (Transformation|SetRelativeScale3D _particlesystem (* (Variables|/Script/Engine.SceneComponent|GetRelativeScale3D _particlesystem) (/ _range 64.0))))