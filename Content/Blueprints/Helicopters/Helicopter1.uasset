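; Player-controlled helicopter prototype that flies by applying physics force to its Driver component.
; Each tick pushes Driver along the actor's up vector with an acceleration scaled by Trottle, so mass is ignored.
; GoForward steps Trottle within a 0–100 range and prints it on screen.
; LookRight, LookUp and GoRight rotate Driver locally in pitch, roll and yaw respectively, using raw axis values without delta-time scaling.
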(event EventTick
  (params (DeltaSeconds :type Float%20%28single-precision%29))
  (Physics|AddForce (Variables|Default|Getdriver) (* (Transformation|GetActorUpVector) (* (Variables|Default|Gettrottle) 2e+01)) "None" true))

(event Input|AxisEvents|InputAxisLookRight
  (params (AxisValue :type Float%20%28single-precision%29))
  (Transformation|AddLocalRotation (Variables|Default|Getdriver) (Math|Rotator|MakeRotator 0.0 AxisValue 0.0) false false))

(event Input|AxisEvents|InputAxisLookUp
  (params (AxisValue :type Float%20%28single-precision%29))
  (Transformation|AddLocalRotation (Variables|Default|Getdriver) (Math|Rotator|MakeRotator AxisValue 0.0 0.0) false false))

(event Input|AxisEvents|InputAxisGoRight
  (params (AxisValue :type Float%20%28single-precision%29))
  (Transformation|AddLocalRotation (Variables|Default|Getdriver) (Math|Rotator|MakeRotator 0.0 0.0 AxisValue) false false))

(event Input|AxisEvents|InputAxisGoForward
  (params (AxisValue :type Float%20%28single-precision%29))
  (if (not (or (> (+ (Variables|Default|Gettrottle) AxisValue) 1e+02) (< (+ (Variables|Default|Gettrottle) AxisValue) 0.0)))
    (bind _output_get (Variables|Default|Settrottle (+ (stale _output_get) AxisValue)))
    (Development|PrintString (Utilities|String|ToString(Float) _output_get) true true "(R=0.000000,G=0.660000,B=1.000000,A=1.000000)" 0.05)))

(fn ConstructionScript)