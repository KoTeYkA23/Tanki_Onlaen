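; Obstacle post with a spotlight that breaks loose and goes dark the first time something overlaps or hits it.
; Both events share one path, latched by a Simulate flag, that turns on physics for the Stolb component, pushes it along HitNormal as an acceleration and hides the light.
; The push direction comes from the Hit event's output, which the overlap event does not supply.
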(event Collision|EventHit
  (params (MyComp :type Primitive%20Component%20Object%20Reference) (Other :type Actor%20Object%20Reference) (OtherComp :type Primitive%20Component%20Object%20Reference) (bSelfMoved :type Boolean) (HitLocation :type Vector :default "0, 0, 0") (HitNormal :type Vector :default "0, 0, 0") (NormalImpulse :type Vector :default "0, 0, 0") (Hit :type Hit%20Result%20Structure%20%28by%20ref%29))
  (bind _stolb (Variables|Default|Getstolb))
  (if (not (Variables|Default|Getsimulate))
    (Variables|Default|Setsimulate true)
    (Physics|SetSimulatePhysics _stolb true)
    (Physics|AddForce _stolb (* HitNormal 1e+02) "None" true)
    (Rendering|SetVisibility (Variables|Default|GetSpotLight) false true)))

(event Collision|EventActorBeginOverlap
  (params (OtherActor :type Actor%20Object%20Reference))
  (bind _stolb (Variables|Default|Getstolb))
  (if (not (Variables|Default|Getsimulate))
    (Variables|Default|Setsimulate true)
    (Physics|SetSimulatePhysics _stolb true)
    (Physics|AddForce _stolb (* (stale Collision|EventHit HitNormal) 1e+02) "None" true)
    (Rendering|SetVisibility (Variables|Default|GetSpotLight) false true)))

(fn ConstructionScript)