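; Player-controlled multiplayer tank with an aimable turret and cannon, cooldown-limited shell fire, HP and death.
; Drives by applying torque to physics-simulated bones, steering by opposing torque on two bone groups.
; Paired client/server events manually mirror pose, firing and HP, while Tick turns the HP text toward the camera and projects the cannon trace onto the HUD crosshair.
; Snaryad overlaps deal damage; death rusts the meshes, starts fire and later possesses a spectator.
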(event Custom|reload%20cooldown
  (Utilities|FlowControl|Delay 2.0)
  (Variables|Default|Setcan%20fire true))

(event Custom|hit
  (params (actor :type Actor%20Object%20Reference))
  (if (and (== (Utilities|GetClass actor) "/Game/Blueprints/Tanks/snaryad.snaryad_C") (!= actor (Variables|Default|Getcurrent_snaryad)))
    (bind _output_get (Variables|Default|SetHP (- (stale _output_get) 5.0)))
    (if (<= _output_get 0.0)
      (Variables|Default|Setdead true)
      (Networking|SwitchHasAuthority
        (:Authority
          (CallFunction|DeadEventServer))
        (:Remote
          (CallFunction|DeadEventClient)))
      (else
        (Networking|SwitchHasAuthority
          (:Authority
            (CallFunction|UpdateHudtoClient _output_get))
          (:Remote
            (CallFunction|UpdateHudtoServer _output_get)))))))

(event Custom|update%20pose%20to%20client
  (params (pos :type Vector) (rot :type Rotator) (bashnya%20rot :type Rotator) (cannon%20rot :type Rotator))
  (bind _tank_mesh (Variables|Default|Gettank%20mesh))
  (Transformation|SetWorldLocation _tank_mesh pos false true)
  (Transformation|SetWorldRotation _tank_mesh rot false true)
  (Transformation|SetRelativeRotation (Variables|Default|Getbashnya) bashnya%20rot false false)
  (Transformation|SetRelativeRotation (Variables|Default|Getpushka) cannon%20rot false false))

(event Custom|update%20pose%20to%20server
  (params (pos :type Vector) (rot :type Rotator) (bashnya%20rot :type Rotator) (cannon%20rot :type Rotator))
  (bind _tank_mesh (Variables|Default|Gettank%20mesh))
  (Transformation|SetWorldLocation _tank_mesh pos false true)
  (Transformation|SetWorldRotation _tank_mesh rot false true)
  (Transformation|SetRelativeRotation (Variables|Default|Getbashnya) bashnya%20rot false false)
  (Transformation|SetRelativeRotation (Variables|Default|Getpushka) cannon%20rot false false))

(event Custom|fire%20from%20client
  (bind _pushka (Variables|Default|Getpushka))
  (bind _returnvalue (Transformation|GetWorldRotation _pushka))
  (CallFunction|FirefromServer2)
  (if (stale _output_get)
    (bind _output_get (Variables|Default|Setcan%20fire false))
    (bind _returnvalue_2 (Game|SpawnActorfromClass "/Game/Blueprints/Tanks/snaryad.snaryad_C" (Math|Transform|MakeTransform (Transformation|GetWorldLocation (Variables|Default|Getfire%20point)) (Math|Rotator|MakeRotator 0.0 (* (.roll _returnvalue) -1.0) (+ (.yaw _returnvalue) 9e+01)) "1,1,1") "AlwaysSpawn" self 0))
    (Variables|Default|Setcurrent_snaryad _returnvalue_2)
    (CallFunction|ReloadCooldown)
    (Components|Activation|Activate (Variables|Default|GetfireParticle) true)))

(event Custom|fire%20from%20server
  (bind _pushka (Variables|Default|Getpushka))
  (bind _returnvalue (Transformation|GetWorldRotation _pushka))
  (CallFunction|FirefromClient2)
  (if (stale _output_get)
    (bind _output_get (Variables|Default|Setcan%20fire false))
    (bind _returnvalue_2 (Game|SpawnActorfromClass "/Game/Blueprints/Tanks/snaryad.snaryad_C" (Math|Transform|MakeTransform (Transformation|GetWorldLocation (Variables|Default|Getfire%20point)) (Math|Rotator|MakeRotator 0.0 (* (.roll _returnvalue) -1.0) (+ (.yaw _returnvalue) 9e+01)) "1,1,1") "AlwaysSpawn" self 0))
    (Variables|Default|Setcurrent_snaryad _returnvalue_2)
    (CallFunction|ReloadCooldown)
    (Components|Activation|Activate (Variables|Default|GetfireParticle) true)))

(event Custom|dead_event_client
  (bind _returnvalue (Game|GetInstigatorController))
  (CallFunction|DeadEventServer)
  (Rendering|Material|SetMaterial (Variables|Default|Gettank%20mesh) 0 "/Game/StarterContent/Materials/M_Metal_Rust.M_Metal_Rust")
  (Rendering|SetVisibility (Variables|Default|GetHPRender) false false)
  (Components|Activation|Deactivate (Variables|Default|Getdim))
  (Components|Activation|Activate (Variables|Default|Getfire) true)
  (Utilities|FlowControl|Delay 5.0)
  (Utilities|IsValid _returnvalue
    (:Is%20Valid
      (bind _returnvalue_2 (Game|SpawnActorfromClass "/Game/Blueprints/spectator.spectator_C" (Math|Transform|MakeTransform "0, 0,100.000000") "AlwaysSpawn" 0 0))
      (Pawn|Possess _returnvalue _returnvalue_2))))

(event Custom|dead_event_server
  (bind _returnvalue (Game|GetInstigatorController))
  (Rendering|Material|SetMaterial (Variables|Default|Gettank%20mesh) 0 "/Game/StarterContent/Materials/M_Metal_Rust.M_Metal_Rust")
  (Rendering|SetVisibility (Variables|Default|GetHPRender) false false)
  (Components|Activation|Deactivate (Variables|Default|Getdim))
  (Components|Activation|Activate (Variables|Default|Getfire) true)
  (Utilities|FlowControl|Delay 5.0)
  (Utilities|IsValid _returnvalue
    (:Is%20Valid
      (bind _returnvalue_2 (Game|SpawnActorfromClass "/Game/Blueprints/spectator.spectator_C" (Math|Transform|MakeTransform "0, 0,100.000000") "AlwaysSpawn" 0 0))
      (Pawn|Possess _returnvalue _returnvalue_2))))

(event Custom|update%20hud%20to%20server2
  (params (hp :type Float%20%28single-precision%29))
  (CallFunction|UpdateHP hp))

(event Custom|update%20hud%20to%20server
  (params (hp :type Float%20%28single-precision%29))
  (CallFunction|UpdateHP hp)
  (CallFunction|UpdateHudtoClient2 hp))

(event Custom|update%20hud%20to%20client
  (params (hp :type Float%20%28single-precision%29))
  (CallFunction|UpdateHP hp)
  (CallFunction|UpdateHudtoServer2 hp))

(event Custom|go%20right
  (params (axis :type Float%20%28single-precision%29))
  (bind _tank_mesh (Variables|Default|Gettank%20mesh))
  (bind _tank_mesh_2 (Variables|Default|Gettank%20mesh))
  (if (!= axis 0.0)
    (for _index (range 3 6)
      (Class|PrimitiveComponent|AddTorqueinDegrees _tank_mesh_2 (Math|Vector|Lerp(Vector) "0, 0, 0" (* (Math|Vector|GetForwardVector _tank_mesh_2) (* (* (Math|Float|Clamp(Float) axis -1.0) -3.0) (Variables|Default|Gettank_power))) 0.1) (Utilities|String|StringToName (Utilities|String|Append "Bone_" (Utilities|String|ToString(Text) (Utilities|Text|ToText(Integer) _index false true 3)))) true)
      (for _index_2 (range 7 10)
        (Class|PrimitiveComponent|AddTorqueinDegrees _tank_mesh (Math|Vector|Lerp(Vector) "0, 0, 0" (* (Math|Vector|GetForwardVector _tank_mesh) (* (* (Math|Float|Clamp(Float) axis -1.0) 3.0) (Variables|Default|Gettank_power))) 0.1) (Utilities|String|StringToName (Utilities|String|Append "Bone_" (Utilities|String|ToString(Text) (Utilities|Text|ToText(Integer) _index_2 false true 3)))) true)))))

(event Custom|go%20fowrard
  (params (axis :type Float%20%28single-precision%29))
  (bind _tank_mesh (Variables|Default|Gettank%20mesh))
  (if (!= axis 0.0)
    (for _index (range 3 10)
      (Class|PrimitiveComponent|AddTorqueinDegrees _tank_mesh (Math|Vector|Lerp(Vector) "0, 0, 0" (* (Math|Vector|GetForwardVector _tank_mesh) (* (* (Math|Float|Clamp(Float) axis -1.0) -2.0) (Variables|Default|Gettank_power))) 0.1) (Utilities|String|StringToName (Utilities|String|Append "Bone_" (Utilities|String|ToString(Text) (Utilities|Text|ToText(Integer) _index false true 3)))) true))))

(event Custom|update%20hud%20to%20client2
  (params (hp :type Float%20%28single-precision%29))
  (CallFunction|UpdateHP hp))

(event Custom|fire%20from%20client2
  (bind _pushka (Variables|Default|Getpushka))
  (bind _returnvalue (Transformation|GetWorldRotation _pushka))
  (if (stale _output_get)
    (bind _output_get (Variables|Default|Setcan%20fire false))
    (bind _returnvalue_2 (Game|SpawnActorfromClass "/Game/Blueprints/Tanks/snaryad.snaryad_C" (Math|Transform|MakeTransform (Transformation|GetWorldLocation (Variables|Default|Getfire%20point)) (Math|Rotator|MakeRotator 0.0 (* (.roll _returnvalue) -1.0) (+ (.yaw _returnvalue) 9e+01)) "1,1,1") "AlwaysSpawn" self 0))
    (Variables|Default|Setcurrent_snaryad _returnvalue_2)
    (CallFunction|ReloadCooldown)
    (Components|Activation|Activate (Variables|Default|GetfireParticle) true)))

(event Custom|fire%20from%20server2
  (bind _pushka (Variables|Default|Getpushka))
  (bind _returnvalue (Transformation|GetWorldRotation _pushka))
  (if (stale _output_get)
    (bind _output_get (Variables|Default|Setcan%20fire false))
    (bind _returnvalue_2 (Game|SpawnActorfromClass "/Game/Blueprints/Tanks/snaryad.snaryad_C" (Math|Transform|MakeTransform (Transformation|GetWorldLocation (Variables|Default|Getfire%20point)) (Math|Rotator|MakeRotator 0.0 (* (.roll _returnvalue) -1.0) (+ (.yaw _returnvalue) 9e+01)) "1,1,1") "AlwaysSpawn" self 0))
    (Variables|Default|Setcurrent_snaryad _returnvalue_2)
    (CallFunction|ReloadCooldown)
    (Components|Activation|Activate (Variables|Default|GetfireParticle) true)))

(event EventTick
  (params (DeltaSeconds :type Float%20%28single-precision%29))
  (bind _hprender (Variables|Default|GetHPRender))
  (bind _tank_mesh (Variables|Default|Gettank%20mesh))
  (bind _bashnya (Variables|Default|Getbashnya))
  (bind _pushka (Variables|Default|Getpushka))
  (bind _pushka_2 (Variables|Default|Getpushka))
  (bind _returnvalue (Transformation|GetWorldLocation _tank_mesh))
  (bind _returnvalue_2 (Transformation|GetWorldRotation _tank_mesh))
  (bind _returnvalue_3 (Transformation|GetWorldLocation _pushka_2))
  (bind _relativerotation (Variables|/Script/Engine.SceneComponent|GetRelativeRotation _bashnya))
  (bind _relativerotation_2 (Variables|/Script/Engine.SceneComponent|GetRelativeRotation _pushka))
  (Utilities|IsValid _hprender
    (:Is%20Valid
      (Transformation|SetWorldRotation _hprender (Math|Rotator|FindLookatRotation (Transformation|GetWorldLocation _hprender) (Transformation|GetWorldLocation (Variables|/Script/Engine.Actor|GetRootComponent (Game|GetPlayerCameraManager 0)))) false false)
      (bind _outhit (Collision|LineTraceForObjects _returnvalue_3 (+ (* (Math|Vector|GetRightVector _pushka_2) 1e+06) _returnvalue_3) (Utilities|Array|MakeArray "ObjectTypeQuery1" "ObjectTypeQuery2" "ObjectTypeQuery3" "ObjectTypeQuery4" "ObjectTypeQuery5" "ObjectTypeQuery6") false 0 "None"))
      (Utilities|IsValid (stale EventBeginPlay _returnvalue)
        (:Is%20Valid
          (Class|Widget|SetRenderTransform (Variables|/Game/Blueprints/UI/Main_HUD.Main_HUD_C|GetImage_48 (stale EventBeginPlay _returnvalue)) (Utilities|Struct|MakeWidgetTransform (.ScreenPosition (Class|WidgetLayoutLibrary|ProjectWorldLocationtoWidgetPosition (Game|GetPlayerController 0) (.Location (Collision|BreakHitResult _outhit))))))
          (Networking|SwitchHasAuthority
            (:Authority
              (Utilities|FlowControl|Delay 0.1)
              (CallFunction|UpdatePosetoClient _returnvalue _returnvalue_2 _relativerotation _relativerotation_2)
              (CallFunction|UpdateHudtoClient (Variables|Default|GetHP)))
            (:Remote
              (CallFunction|UpdatePosetoServer _returnvalue _returnvalue_2 _relativerotation _relativerotation_2))))))))

(event EventBeginPlay
  (Class|SkeletalMeshComponent|SetAllBodiesSimulatePhysics (Variables|Default|Gettank%20mesh) true)
  (bind _returnvalue (UserInterface|CreateWidget "/Game/Blueprints/UI/Main_HUD.Main_HUD_C" (Game|GetPlayerController 0)))
  (Utilities|IsValid _returnvalue
    (:Is%20Valid
      (UserInterface|Viewport|AddtoViewport _returnvalue 0)
      (CallFunction|UpdateHP (Variables|Default|GetHP)))))

(event Collision|EventActorBeginOverlap
  (params (OtherActor :type Actor%20Object%20Reference))
  (if (!= (Variables|Default|Getcurrent_snaryad) OtherActor)
    (CallFunction|Hit OtherActor)))

(event Input|ActionEvents|InputActionfire
  (params (Key :type Key%20Structure))
  (:Pressed
    (if (not (Variables|Default|Getdead))
      (CallFunction|FirefromClient)
      (CallFunction|FirefromServer))))

(event Input|AxisEvents|InputAxisLookRight
  (params (AxisValue :type Float%20%28single-precision%29))
  (if (not (Variables|Default|Getdead))
    (if (not (or (> (+ (* AxisValue -1.0) (stale _output_get)) 9e+01) (< (+ (* AxisValue -1.0) (stale _output_get)) -9e+01)))
      (bind _output_get (Variables|Default|Setupratio (+ (* AxisValue -1.0) (stale _output_get))))
      (Transformation|SetRelativeRotation (Variables|Default|Getcamera%20arm) (Math|Rotator|MakeRotator 0.0 _output_get 9e+01) false false)
      (if (Math|Float|InRange(Float) (* (+ _output_get 15.0) -1.0) -25.0 1e+01)
        (Transformation|SetRelativeRotation (Variables|Default|Getpushka) (Math|Rotator|MakeRotator (* (+ _output_get 15.0) -1.0) 0.0 0.0) false false)
        (Variables|Default|Setupratio_cannon (+ _output_get 15.0))))))

(event Input|AxisEvents|InputAxisGoRight
  (params (AxisValue :type Float%20%28single-precision%29))
  (if (not (Variables|Default|Getdead))
    (CallFunction|GoRight AxisValue)))

(event Input|AxisEvents|InputAxisLookUp
  (params (AxisValue :type Float%20%28single-precision%29))
  (if (not (Variables|Default|Getdead))
    (Transformation|AddRelativeRotation (Variables|Default|Getbashnya) (Math|Rotator|MakeRotator 0.0 0.0 AxisValue) false false)))

(event Input|AxisEvents|InputAxisGoForward
  (params (AxisValue :type Float%20%28single-precision%29))
  (if (not (Variables|Default|Getdead))
    (CallFunction|GoFowrard AxisValue)))

(fn ConstructionScript)

(fn UpdateHP
  (params (hp :type Float%20%28single-precision%29))
  (Rendering|Components|TextRender|SetText (Variables|Default|GetHPRender) (Utilities|Text|FormatText "{value}:HP" hp)))