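; Tank bullet projectile built from cylinder and cone meshes, with projectile movement, a tail effect and an explosion effect.
; An overlap activates the explosion only when the other actor's class is exactly Tank1.
; Any overlap or hit then stops movement, hides the meshes, disables their collision and switches off the tail.
; The actor destroys itself after a delay rather than immediately on impact.
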(event Collision|EventActorBeginOverlap
  (params (OtherActor :type Actor%20Object%20Reference))
  (if (!= (Utilities|GetClass OtherActor) "/Game/Blueprints/Tanks/Tank1.Tank1_C")
    _
    (else
      (Components|Activation|Activate (Variables|Default|Getexplode) true)))
  (Components|Activation|Deactivate (Variables|Default|GetProjectileMovement))
  (Collision|SetCollisionEnabled (Variables|Default|GetCylinder) "NoCollision")
  (Rendering|SetVisibility (Variables|Default|GetCone) false false)
  (Components|Activation|Deactivate (Variables|Default|Gettail))
  (Utilities|FlowControl|Delay 15.0)
  (Actor|DestroyActor))

(event Collision|EventHit
  (params (MyComp :type Primitive%20Component%20Object%20Reference) (Other :type Actor%20Object%20Reference) (OtherComp :type Primitive%20Component%20Object%20Reference) (bSelfMoved :type Boolean) (HitLocation :type Vector :default "0, 0, 0") (HitNormal :type Vector :default "0, 0, 0") (NormalImpulse :type Vector :default "0, 0, 0") (Hit :type Hit%20Result%20Structure%20%28by%20ref%29))
  (Components|Activation|Deactivate (Variables|Default|GetProjectileMovement))
  (Collision|SetCollisionEnabled (Variables|Default|GetCylinder) "NoCollision")
  (Rendering|SetVisibility (Variables|Default|GetCone) false false)
  (Components|Activation|Deactivate (Variables|Default|Gettail))
  (Utilities|FlowControl|Delay 15.0)
  (Actor|DestroyActor))

(fn ConstructionScript)