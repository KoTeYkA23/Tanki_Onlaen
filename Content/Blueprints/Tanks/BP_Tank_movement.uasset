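; Tank movement Blueprint that drives a physics-simulated tank by applying torque to its left and right wheel bones from forward and right axis inputs.
; Forward input torques both sides together, scaled by a power curve sampled at the mesh's current speed.
; Right input torques the sides in opposite directions for skid steering, using a fixed curve sample.
; Zero input leads to a shared braking branch that counters each wheel's angular velocity.
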(event Custom|Move_forward
  (params (Axis :type Float%20%28single-precision%29))
  (bind _mesh (Variables|Default|GetMesh))
  (bind _mesh_2 (Variables|Default|GetMesh))
  (bind _result (Math|Float|NegateFloat Axis)
    (:%20%20
      (if (!= Axis 0.0)
        (for _array_element (Variables|Default|GetLeft%20Wheels)
          (Class|PrimitiveComponent|AddTorqueinDegrees _mesh (* (Math|Vector|GetForwardVector (Variables|Default|GetMesh)) (* (* (Math|Curves|GetFloatValue (Variables|Default|Getcurve%20power) (Math|Vector|VectorLength (Transformation|GetComponentVelocity (Variables|Default|GetMesh)))) 5e+03) _result)) _array_element true))
        (for _array_element_2 (Variables|Default|GetRight%20Wheels)
          (Class|PrimitiveComponent|AddTorqueinDegrees _mesh (* (Math|Vector|GetForwardVector (Variables|Default|GetMesh)) (* (* (Math|Curves|GetFloatValue (Variables|Default|Getcurve%20power) (Math|Vector|VectorLength (Transformation|GetComponentVelocity (Variables|Default|GetMesh)))) 5e+03) _result)) _array_element_2 true))
        (elif (and (== Axis 0.0) (== (stale Custom|Move_right Axis) 0.0))
          (for _array_element_3 (Variables|Default|GetLeft%20Wheels)
            (Class|PrimitiveComponent|AddTorqueinDegrees _mesh_2 (* (Physics|GetPhysicsAngularVelocityinDegrees _mesh_2 _array_element_3) -15.0) _array_element_3 true))
          (for _array_element_4 (Variables|Default|GetRight%20Wheels)
            (Class|PrimitiveComponent|AddTorqueinDegrees _mesh_2 (* (Physics|GetPhysicsAngularVelocityinDegrees _mesh_2 _array_element_4) -15.0) _array_element_4 true)))))))

(event Custom|Move_right
  (params (Axis :type Float%20%28single-precision%29))
  (bind _curve_power (Variables|Default|Getcurve%20power))
  (bind _mesh (Variables|Default|GetMesh))
  (bind _returnvalue (Math|Curves|GetFloatValue _curve_power 3e+02))
  (bind _returnvalue_2 (* _returnvalue 5e+03))
  (if (!= Axis 0.0)
    (for _array_element (Variables|Default|GetLeft%20Wheels)
      (Class|PrimitiveComponent|AddTorqueinDegrees (Variables|Default|GetMesh) (* (Math|Vector|GetForwardVector (Variables|Default|GetMesh)) (* (* _returnvalue_2 -2.0) Axis)) _array_element true))
    (for _array_element_2 (Variables|Default|GetRight%20Wheels)
      (Class|PrimitiveComponent|AddTorqueinDegrees (Variables|Default|GetMesh) (* (Math|Vector|GetForwardVector (Variables|Default|GetMesh)) (* (* _returnvalue_2 2.0) Axis)) _array_element_2 true))
    (elif (and (== (stale Custom|Move_forward Axis) 0.0) (== Axis 0.0))
      (for _array_element_3 (Variables|Default|GetLeft%20Wheels)
        (Class|PrimitiveComponent|AddTorqueinDegrees _mesh (* (Physics|GetPhysicsAngularVelocityinDegrees _mesh _array_element_3) -15.0) _array_element_3 true))
      (for _array_element_4 (Variables|Default|GetRight%20Wheels)
        (Class|PrimitiveComponent|AddTorqueinDegrees _mesh (* (Physics|GetPhysicsAngularVelocityinDegrees _mesh _array_element_4) -15.0) _array_element_4 true)))))