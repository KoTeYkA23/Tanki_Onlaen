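; Component that syncs a tank's physics mesh across the network, with the locally controlled pawn as the source of movement.
; Every tick that pawn sends mesh location, rotation and velocity, straight to the client event with authority, otherwise through the server event, which applies and forwards them.
; Non-locally controlled copies teleport the mesh to the received pose and overwrite its linear velocity, with no interpolation.
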(event Custom|update%20pose%20to%20client
  (params (pos :type Vector) (rot :type Rotator) (velocity :type Vector))
  (bind _mesh (Variables|Default|GetMesh))
  (Utilities|IsValid _mesh
    (:Is%20Valid
      (if (not (Pawn|IsLocallyControlled (.AsPawn (Utilities|Casting|CastToPawn (Components|GetOwner)))))
        (Transformation|SetWorldLocationAndRotation _mesh pos rot false true)
        (Physics|SetPhysicsLinearVelocity _mesh velocity false "None")))))

(event Custom|update%20pos%20to%20server
  (params (pos :type Vector) (rot :type Rotator) (Velocity :type Vector))
  (bind _mesh (Variables|Default|GetMesh))
  (Utilities|IsValid _mesh
    (:Is%20Valid
      (if (not (Pawn|IsLocallyControlled (.AsPawn (Utilities|Casting|CastToPawn (Components|GetOwner)))))
        (Transformation|SetWorldLocationAndRotation _mesh pos rot false true)
        (Physics|SetPhysicsLinearVelocity _mesh Velocity false "None")
        (CallFunction|UpdatePosetoClient pos rot Velocity)))))

(event EventTick
  (params (DeltaSeconds :type Float%20%28single-precision%29))
  (bind _returnvalue (Components|GetOwner))
  (bind _mesh (Variables|Default|GetMesh))
  (bind _returnvalue_2 (Transformation|GetWorldLocation _mesh))
  (bind _returnvalue_3 (Transformation|GetWorldRotation _mesh))
  (bind _returnvalue_4 (Transformation|GetComponentVelocity _mesh))
  (bind _aspawn (Utilities|Casting|CastToPawn _returnvalue))
  (if (Pawn|IsLocallyControlled _aspawn)
    (if (Ability|HasAuthority _returnvalue)
      (CallFunction|UpdatePosetoClient _returnvalue_2 _returnvalue_3 _returnvalue_4)
      (else
        (CallFunction|UpdatePostoServer _returnvalue_2 _returnvalue_3 _returnvalue_4)))))