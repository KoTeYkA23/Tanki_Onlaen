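; Tank shell projectile that reacts to the first actors it overlaps by stopping and hiding itself.
; The Explode effect activates only when the overlapped actor's class is Tank1, and no damage is applied here.
; Any overlap halts projectile movement, disables collision on the cylinder and cone meshes, hides them and deactivates the Tail effect.
; The actor destroys itself after a delay.
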(event Collision|EventActorBeginOverlap
  (params (OtherActor :type Actor%20Object%20Reference))
  (if (!= (Utilities|GetClass OtherActor) "/Game/Blueprints/Tanks/Tank1.Tank1_C")
    _
    (else
      (Components|Activation|Activate (Variables|Default|Getexplode) true)))
  (Game|Components|ProjectileMovement|StopSimulating (Variables|Default|GetProjectileMovement) (Collision|MakeHitResult false false 0.0 0.0 "0, 0, 0" "0, 0, 0" "0,0,1" "0,0,1" 0 0))
  (Collision|SetCollisionEnabled (Variables|Default|GetCylinder) "NoCollision")
  (Rendering|SetVisibility (Variables|Default|GetCone) false false)
  (Components|Activation|Deactivate (Variables|Default|Gettail))
  (Utilities|FlowControl|Delay 15.0)
  (Actor|DestroyActor))

(fn ConstructionScript)