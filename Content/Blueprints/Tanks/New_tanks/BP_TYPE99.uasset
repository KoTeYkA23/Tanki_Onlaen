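; BP_TYPE99 is the player-controllable Type 99 tank.
; On BeginPlay it hands its Type99 mesh to the BPTankMovement and BPTankReplicate components and enables physics simulation on the "Korpus" bone and all bodies below it.
; Drive axes forward to BPTankMovement, while look axes feed controller rotation, with LookUp driving yaw and LookRight driving pitch despite their names.
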(event EventBeginPlay
  (bind _type_99 (Variables|Default|GetType_99))
  (Variables|/Game/Blueprints/Tanks/BP_Tank_movement.BP_Tank_movement_C|SetMesh (Variables|Default|GetBP_Tank_movement) _type_99)
  (Variables|/Game/Blueprints/Tanks/BP_Tank_replicate.BP_Tank_replicate_C|SetMesh (Variables|Default|GetBP_Tank_replicate) _type_99)
  (Class|SkeletalMeshComponent|SetAllBodiesBelowSimulatePhysics _type_99 (Utilities|String|StringToName "Korpus") true true))

(event Input|AxisEvents|InputAxisLookUp
  (params (AxisValue :type Float%20%28single-precision%29))
  (Pawn|Input|AddControllerYawInput AxisValue))

(event Input|AxisEvents|InputAxisLookRight
  (params (AxisValue :type Float%20%28single-precision%29))
  (Pawn|Input|AddControllerPitchInput AxisValue))

(event Input|AxisEvents|InputAxisGoForward
  (params (AxisValue :type Float%20%28single-precision%29))
  (Default|MoveForward (Variables|Default|GetBP_Tank_movement) AxisValue))

(event Input|AxisEvents|InputAxisGoRight
  (params (AxisValue :type Float%20%28single-precision%29))
  (Default|MoveRight (Variables|Default|GetBP_Tank_movement) AxisValue))

(fn ConstructionScript)